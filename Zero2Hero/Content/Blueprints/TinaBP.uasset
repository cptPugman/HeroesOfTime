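; Twin-stick shooter player character (Tina) that spawns with a pistol and HUD, giving player 0 its own material and spawn offset.
; Stick aim rotates and fires, while two inputs cycle Metralleta, Pistola and Shotgun by respawning the socketed actor.
; Taunts destroy the weapon; movement and Tick logic respawn weapons and clear taunt flags.
; On death it disables input, asks TwinStickMode to respawn after a delay, then destroys itself.
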(event `self.ReceiveBeginPlay`
  (bind _mesh (`self.Mesh`))
  (if (== (`self.GetController`) (`GameplayStatics.GetPlayerController` 0))
    (`PrimitiveComponent.SetMaterial` (`self.Mesh`) 0 "/Game/StarterContent/Materials/M_Tech_Hex_Tile.M_Tech_Hex_Tile"))
  (if (== (`self.GetController`) (`GameplayStatics.GetPlayerController` 0))
    (`self.K2_AddActorLocalOffset` (0.0 200.0 0.0)))
  (`|ExecutionSequence`
    (:`then_0`
      (bind _returnvalue (`|SpawnActorFromClass` "/Game/Blueprints/Armas/Pistola.Pistola_C" (`SceneComponent.K2_GetComponentToWorld` _mesh) "Undefined" "OverrideRootScale"))
      (bind _output_get (set `self.Weapon` _returnvalue))
      (`self.K2_AttachRootComponentTo` _output_get _mesh "GunSocket" "SnapToTarget" true))
    (:`then_1`
      (bind _astwin_stick_mode (cast `/Game/Blueprints/TwinStickMode` (`GameplayStatics.GetGameMode`)))
      (bind _output_get_2 (set `self.GameMode` _astwin_stick_mode))
      (set `/Game/Blueprints/TwinStickMode.PlayerSpawnTransform` (`self.GetTransform`) _output_get_2))
    (:`then_2`
      (bind _returnvalue_2 (`|CreateWidget` "/Game/Blueprints/TwinStickHUD.TwinStickHUD_C"))
      (`UserWidget.AddToViewport` _returnvalue_2 0))))

(event `InputAxis|MoveUp`
  (params (AxisValue :type "Float (single-precision)"))
  (bind _returnvalue (`SceneComponent.K2_GetComponentToWorld` (`self.Mesh`)))
  ;[1 1 1] Movement
  (if (> AxisValue 0.0)
    (if (`self.weaponDestroyed`)
      (if (== (`self.counterArmas`) 0)
        (bind _returnvalue_2 (`|SpawnActorFromClass` "/Game/Blueprints/Armas/Metralleta.Metralleta_C" _returnvalue "Undefined" "OverrideRootScale"))
        (bind _output_get (set `self.Weapon` _returnvalue_2))
        (`self.K2_AttachRootComponentTo` _output_get (`self.Mesh`) "GunSocket" "SnapToTarget" true)
        (set `self.taunting` false :!label _label)
        (set `self.dancing` false)
        (set `self.standing` false)
        (set `self.laughing` false)
        (set `self.taunts` false)
        (`self.AddMovementInput` (1.0 0.0 0.0) AxisValue :!label _label_2)
        (elif (== (`self.counterArmas`) 1)
          (bind _returnvalue_3 (`|SpawnActorFromClass` "/Game/Blueprints/Armas/Pistola.Pistola_C" _returnvalue "Undefined" "OverrideRootScale"))
          (bind _output_get_2 (set `self.Weapon` _returnvalue_3))
          (`self.K2_AttachRootComponentTo` _output_get_2 (`self.Mesh`) "GunSocket" "SnapToTarget" true)
          (goto _label)
          (elif (== (`self.counterArmas`) 2)
            (bind _returnvalue_4 (`|SpawnActorFromClass` "/Game/Blueprints/Armas/Shotgun.Shotgun_C" _returnvalue "Undefined" "OverrideRootScale"))
            (bind _output_get_3 (set `self.Weapon` _returnvalue_4))
            (`self.K2_AttachRootComponentTo` _output_get_3 (`self.Mesh`) "GunSocket" "SnapToTarget" true)
            (goto _label))))
      (else
        (goto _label)))
    (else
      (goto _label_2))))

(event `InputAxis|LookUp`
  (params (AxisValue :type "Float (single-precision)"))
  (bind _weapon (`self.Weapon`))
  ;[1 1 1] Rotation
  (bind _returnvalue (`KismetMathLibrary.MakeVector` AxisValue (stale `InputAxis|LookRight` AxisValue)))
  (if (> (`KismetMathLibrary.VSize` _returnvalue) 0.25) :!label _label_3
    (`Controller.SetControlRotation` (`self.GetController`) (`KismetMathLibrary.Conv_VectorToRotator` _returnvalue))
    ;[1 0.365 0.365] Para Saber Quien dispara
    (if (== (`self.GetController`) (`GameplayStatics.GetPlayerController` 0))
      (`/Game/Blueprints/Armas/Weapon.PullTrigger` _weapon 0)
      (else
        (`/Game/Blueprints/Armas/Weapon.PullTrigger` _weapon 1)))
    (else
      (`/Game/Blueprints/Armas/Weapon.ReleaseTrigger` _weapon))))

(event `InputAxis|LookRight`
  (params (AxisValue :type "Float (single-precision)"))
  ;[1 1 1] Rotation
  (goto _label_3))

(event `InputAxis|MoveRight`
  (params (AxisValue :type "Float (single-precision)"))
  (bind _returnvalue (`SceneComponent.K2_GetComponentToWorld` (`self.Mesh`)))
  ;[1 1 1] Movement
  (if (> AxisValue 0.0)
    (if (`self.weaponDestroyed`)
      (if (== (`self.counterArmas`) 0)
        (bind _returnvalue_2 (`|SpawnActorFromClass` "/Game/Blueprints/Armas/Metralleta.Metralleta_C" _returnvalue "Undefined" "OverrideRootScale"))
        (bind _output_get (set `self.Weapon` _returnvalue_2))
        (`self.K2_AttachRootComponentTo` _output_get (`self.Mesh`) "GunSocket" "SnapToTarget" true)
        (set `self.taunting` false :!label _label_4)
        (set `self.dancing` false)
        (set `self.standing` false)
        (set `self.laughing` false)
        (set `self.taunts` false)
        (`self.AddMovementInput` (0.0 1.0 0.0) AxisValue :!label _label_5)
        (elif (== (`self.counterArmas`) 1)
          (bind _returnvalue_3 (`|SpawnActorFromClass` "/Game/Blueprints/Armas/Pistola.Pistola_C" _returnvalue "Undefined" "OverrideRootScale"))
          (bind _output_get_2 (set `self.Weapon` _returnvalue_3))
          (`self.K2_AttachRootComponentTo` _output_get_2 (`self.Mesh`) "GunSocket" "SnapToTarget" true)
          (goto _label_4)
          (elif (== (`self.counterArmas`) 2)
            (bind _returnvalue_4 (`|SpawnActorFromClass` "/Game/Blueprints/Armas/Shotgun.Shotgun_C" _returnvalue "Undefined" "OverrideRootScale"))
            (bind _output_get_3 (set `self.Weapon` _returnvalue_4))
            (`self.K2_AttachRootComponentTo` _output_get_3 (`self.Mesh`) "GunSocket" "SnapToTarget" true)
            (goto _label_4))))
      (else
        (goto _label_4)))
    (else
      (goto _label_5))))

(event `Event Affect Health`
  (params (Delta :type "Float (double-precision)") (player :type Integer))
  (`KismetSystemLibrary.PrintString` (`KismetStringLibrary.Conv_DoubleToString` Delta))
  (`self.CalculateHealth` Delta)
  (if (`self.IsDead`)
    (`self.DisableInput` null)
    (`/Game/Blueprints/Armas/Weapon.ReleaseTrigger` (`self.Weapon`))
    (`KismetSystemLibrary.Delay` 3.0)
    ;[1 1 1] Modificado 08/03
    (`/Game/Blueprints/TwinStickMode.RespawnPlayer` (`self.GameMode`) (`self.GetController`))
    (`self.K2_DestroyActor` (`self.Weapon`))
    (`self.K2_DestroyActor` self)
    (bind _outactors (`GameplayStatics.GetAllActorsOfClass` "/Game/Blueprints/Camera.Camera_C"))
    (`PlayerController.SetViewTargetWithBlend` (`GameplayStatics.GetPlayerController` 0) (`KismetArrayLibrary.Array_Get` _outactors) 0.0 "VTBlend_Linear" 0.0 false)))

(event `InputAction|Taunts`
  (params (Key :type "Key Structure" :default "AnyKey"))
  (:`Pressed`
    (set `self.taunts` true))
  (:`Released`
    (set `self.taunts` false)))

(event `InputAction|Taunt_Dance`
  (params (Key :type "Key Structure" :default "AnyKey"))
  (:`Pressed`
    (`/Game/Blueprints/Armas/Weapon.ReleaseTrigger` (`self.Weapon`))
    (set `self.dancing` true)
    (set `self.taunting` false)
    (set `self.laughing` false)
    (set `self.standing` false)
    (set `self.taunts` true :!label _label_6)
    (`self.K2_DestroyActor` (`self.Weapon`))
    (set `self.weaponDestroyed` true)))

(event `InputAction|Taunt_StandUp`
  (params (Key :type "Key Structure" :default "AnyKey"))
  (:`Pressed`
    (`/Game/Blueprints/Armas/Weapon.ReleaseTrigger` (`self.Weapon`))
    (set `self.standing` true)
    (set `self.taunting` false)
    (set `self.dancing` false)
    (set `self.laughing` false)
    (goto _label_6)))

(event `InputAction|Taunt_Laugh`
  (params (Key :type "Key Structure" :default "AnyKey"))
  (:`Pressed`
    (`/Game/Blueprints/Armas/Weapon.ReleaseTrigger` (`self.Weapon`))
    (set `self.laughing` true)
    (set `self.taunting` false)
    (set `self.dancing` false)
    (set `self.standing` false)
    (goto _label_6)))

(event `InputAction|Taunt_Taunt`
  (params (Key :type "Key Structure" :default "AnyKey"))
  (:`Pressed`
    (`/Game/Blueprints/Armas/Weapon.ReleaseTrigger` (`self.Weapon`))
    (set `self.taunting` true)
    (set `self.dancing` false)
    (set `self.laughing` false)
    (set `self.standing` false)
    (goto _label_6)))

(event `self.ReceiveTick`
  (params (DeltaSeconds :type "Float (single-precision)"))
  (bind _returnvalue (`self.GetInputAxisKeyValue`))
  (bind _returnvalue_2 (`self.GetInputAxisKeyValue`))
  (bind _weapon (`self.Weapon`))
  (bind _returnvalue_3 (`SceneComponent.K2_GetComponentToWorld` (`self.Mesh`)))
  (if (or (or (< _returnvalue -0.2) (> _returnvalue 0.2)) (or (< _returnvalue_2 -0.2) (> _returnvalue_2 0.2)))
    (if (== (`self.player controller`) 0)
      (`self.K2_DestroyActor` _weapon)
      (bind _returnvalue_4 (`|SpawnActorFromClass` "/Game/Blueprints/Armas/Metralleta.Metralleta_C" _returnvalue_3 "Undefined" "OverrideRootScale"))
      (bind _output_get (set `self.Weapon` _returnvalue_4))
      (`self.K2_AttachRootComponentTo` _output_get (`self.Mesh`) "GunSocket" "SnapToTarget" true)
      (set `self.taunting` false :!label _label_7)
      (set `self.dancing` false)
      (set `self.standing` false)
      (set `self.laughing` false)
      (set `self.taunts` false)
      (if (> (`KismetMathLibrary.VSize` (`CharacterMovementComponent.GetCurrentAcceleration` (`self.CharacterMovement`))) 0.0) :!label _label_8
        (set `self.weapon` null)
        (if (or (`self.taunting`) (`self.laughing`) (`self.standing`) (`self.dancing`))
          (set `self.taunting` false)
          (set `self.dancing` false)
          (set `self.laughing` false)
          (set `self.standing` false)))
      (elif (== (`self.player controller`) 1)
        (`self.K2_DestroyActor` _weapon)
        (bind _returnvalue_5 (`|SpawnActorFromClass` "/Game/Blueprints/Armas/Pistola.Pistola_C" _returnvalue_3 "Undefined" "OverrideRootScale"))
        (bind _output_get_2 (set `self.Weapon` _returnvalue_5))
        (`self.K2_AttachRootComponentTo` _output_get_2 (`self.Mesh`) "GunSocket" "SnapToTarget" true)
        (goto _label_7)
        (elif (== (`self.player controller`) 2)
          (`self.K2_DestroyActor` _weapon)
          (bind _returnvalue_6 (`|SpawnActorFromClass` "/Game/Blueprints/Armas/Shotgun.Shotgun_C" _returnvalue_3 "Undefined" "OverrideRootScale"))
          (bind _output_get_3 (set `self.Weapon` _returnvalue_6))
          (`self.K2_AttachRootComponentTo` _output_get_3 (`self.Mesh`) "GunSocket" "SnapToTarget" true)
          (goto _label_7))))
    (else
      (goto _label_8))))

(event `InputAction|Cambio de arma derecha`
  (params (Key :type "Key Structure" :default "AnyKey"))
  (bind _weapon (`self.Weapon`))
  (bind _returnvalue (`SceneComponent.K2_GetComponentToWorld` (`self.Mesh`)))
  (:`Pressed`
    (bind _output_get (set `self.counterArmas` (+ (`self.counterArmas`) 1)))
    (if (== (mod _output_get 3) 0)
      (`self.K2_DestroyActor` _weapon)
      (bind _returnvalue_2 (`|SpawnActorFromClass` "/Game/Blueprints/Armas/Metralleta.Metralleta_C" _returnvalue "Undefined" "OverrideRootScale"))
      (bind _output_get_2 (set `self.Weapon` _returnvalue_2))
      (`self.K2_AttachRootComponentTo` _output_get_2 (`self.Mesh`) "GunSocket" "SnapToTarget" true)
      (elif (== (mod _output_get 3) 1)
        (`self.K2_DestroyActor` _weapon)
        (bind _returnvalue_3 (`|SpawnActorFromClass` "/Game/Blueprints/Armas/Pistola.Pistola_C" _returnvalue "Undefined" "OverrideRootScale"))
        (bind _output_get_3 (set `self.Weapon` _returnvalue_3))
        (`self.K2_AttachRootComponentTo` _output_get_3 (`self.Mesh`) "GunSocket" "SnapToTarget" true)
        (elif (== (mod _output_get 3) 2)
          (`self.K2_DestroyActor` _weapon)
          (bind _returnvalue_4 (`|SpawnActorFromClass` "/Game/Blueprints/Armas/Shotgun.Shotgun_C" _returnvalue "Undefined" "OverrideRootScale"))
          (bind _output_get_4 (set `self.Weapon` _returnvalue_4))
          (`self.K2_AttachRootComponentTo` _output_get_4 (`self.Mesh`) "GunSocket" "SnapToTarget" true))))))

(event `InputAction|Cambio de arma izquierda`
  (params (Key :type "Key Structure" :default "AnyKey"))
  (bind _weapon (`self.Weapon`))
  (bind _returnvalue (`SceneComponent.K2_GetComponentToWorld` (`self.Mesh`)))
  (:`Pressed`
    (bind _output_get (set `self.counterArmas` (+ (`self.counterArmas`) 2)))
    (if (== (mod _output_get 3) 0)
      (`self.K2_DestroyActor` _weapon)
      (bind _returnvalue_2 (`|SpawnActorFromClass` "/Game/Blueprints/Armas/Metralleta.Metralleta_C" _returnvalue "Undefined" "OverrideRootScale"))
      (bind _output_get_2 (set `self.Weapon` _returnvalue_2))
      (`self.K2_AttachRootComponentTo` _output_get_2 (`self.Mesh`) "GunSocket" "SnapToTarget" true)
      (elif (== (mod _output_get 3) 1)
        (`self.K2_DestroyActor` _weapon)
        (bind _returnvalue_3 (`|SpawnActorFromClass` "/Game/Blueprints/Armas/Pistola.Pistola_C" _returnvalue "Undefined" "OverrideRootScale"))
        (bind _output_get_3 (set `self.Weapon` _returnvalue_3))
        (`self.K2_AttachRootComponentTo` _output_get_3 (`self.Mesh`) "GunSocket" "SnapToTarget" true)
        (elif (== (mod _output_get 3) 2)
          (`self.K2_DestroyActor` _weapon)
          (bind _returnvalue_4 (`|SpawnActorFromClass` "/Game/Blueprints/Armas/Shotgun.Shotgun_C" _returnvalue "Undefined" "OverrideRootScale"))
          (bind _output_get_4 (set `self.Weapon` _returnvalue_4))
          (`self.K2_AttachRootComponentTo` _output_get_4 (`self.Mesh`) "GunSocket" "SnapToTarget" true))))))

(fn `UserConstructionScript`
  (`parent.UserConstructionScript`))