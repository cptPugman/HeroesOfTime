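; Actor that draws a particle laser between the two local players and hurts enemies caught in it.
; BeginPlay spawns the second player, finds static mesh actors tagged s1 and s2, and attaches the beam to the players.
; While they are in range, Tick line-traces between them, damaging the enemy hit for both players.
; Excess distance or a failed hero cast moves the beam onto the tagged actors, and a delayed flag pauses reconnection.
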(event `self.ReceiveTick`
  (params (DeltaSeconds :type "Float (single-precision)"))
  (bind _s2 (`self.s2`))
  (cast `/Game/Blueprints/HeroCharacter` (`GameplayStatics.GetPlayerCharacter` 0)
    (:`then`
      (cast `/Game/Blueprints/HeroCharacter` (`GameplayStatics.GetPlayerCharacter` 1)
        (:`then`
          (if (`self.laser`)
            _
            (elif (> (`KismetMathLibrary.VSize` (- (`self.K2_GetActorLocation` (`GameplayStatics.GetPlayerCharacter` 0)) (`self.K2_GetActorLocation` (`GameplayStatics.GetPlayerCharacter` 1)))) 600.0)
              (if (> (`KismetMathLibrary.VSize` (- (`self.K2_GetActorLocation` (`GameplayStatics.GetPlayerCharacter` 0)) (`self.K2_GetActorLocation` (`GameplayStatics.GetPlayerCharacter` 1)))) 600.0)
                (`/Engine/EditorBlueprintResources/StandardMacros.IsValid` (`self.s1`)
                  (:`Is Valid`
                    (`ParticleSystemComponent.SetActorParameter` (`self.ParticleSystem`) "BeamSource" (`self.s1`) :!label _label)
                    (`/Engine/EditorBlueprintResources/StandardMacros.IsValid` _s2
                      (:`Is Valid`
                        (`ParticleSystemComponent.SetActorParameter` (`self.ParticleSystem`) "BeamTarget" _s2)
                        (set `self.laser` true)
                        (`KismetSystemLibrary.Delay` 5.0)
                        (set `self.laser` false))))))
              (else
                (`ParticleSystemComponent.SetActorParameter` (`self.ParticleSystem`) "BeamSource" (`GameplayStatics.GetPlayerCharacter` 0))
                (`ParticleSystemComponent.SetActorParameter` (`self.ParticleSystem`) "BeamTarget" (`GameplayStatics.GetPlayerCharacter` 1))
                (bind _outhit (`KismetSystemLibrary.LineTraceSingle` (`self.K2_GetActorLocation` (`GameplayStatics.GetPlayerCharacter` 0)) (`self.K2_GetActorLocation` (`GameplayStatics.GetPlayerCharacter` 1)) "TraceTypeQuery1"))
                (bind _asenemy_character (cast `/Game/Blueprints/Enemies/EnemyCharacter` (`.HitActor` (`GameplayStatics.BreakHitResult` _outhit))))
                (`/Game/Blueprints/Enemies/EnemyCharacter.AffectHealth` _asenemy_character -3.0 0)
                (`/Game/Blueprints/Enemies/EnemyCharacter.AffectHealth` _asenemy_character -3.0 1)))))
        (:`CastFailed`
          (goto _label))))
    (:`CastFailed`
      (goto _label))))

(event `self.ReceiveBeginPlay`
  (bind _outactors (`GameplayStatics.GetAllActorsOfClass` "/Script/Engine.StaticMeshActor"))
  (for _array_element _outactors
    (if (`self.ActorHasTag` _array_element "s1")
      (set `self.s1` _array_element)
      (elif (`self.ActorHasTag` _array_element "s2")
        (set `self.s2` _array_element))))
  (`GameplayStatics.CreatePlayer` 1)
  (`ParticleSystemComponent.SetActorParameter` (`self.ParticleSystem`) "BeamSource" (`GameplayStatics.GetPlayerCharacter` 0))
  (`ParticleSystemComponent.SetActorParameter` (`self.ParticleSystem`) "BeamTarget" (`GameplayStatics.GetPlayerCharacter` 1)))

(fn `UserConstructionScript`)