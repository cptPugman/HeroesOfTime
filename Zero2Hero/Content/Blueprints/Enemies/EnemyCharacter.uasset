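; Enemy character for a twin-stick game that damages heroes on contact and awards score when killed.
; Overlapping a HeroCharacter starts a looping timer that deals damage at the attack rate until that hero leaves.
; On death it stops attacking, ignores pawn and world-dynamic collision, credits the TwinStickMode score for the given player, detaches its controller and destroys itself after a delay.
; The construction script tints the body through a dynamic material instance.
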(event `/Game/Blueprints/iDamageable.AffectHealth`
  (params (Delta :type "Float (single-precision)") (Player :type Integer))
  (bind _capsulecomponent (`self.CapsuleComponent`))
  (bind _score (`self.Score`))
  (`self.CalculateHealth` Delta)
  (if (`self.IsDead`)
    (`KismetSystemLibrary.K2_ClearTimer` null "DamageTheHero")
    (`PrimitiveComponent.SetCollisionResponseToChannel` _capsulecomponent "ECC_WorldDynamic" "ECR_Ignore")
    (`PrimitiveComponent.SetCollisionResponseToChannel` _capsulecomponent "ECC_Pawn" "ECR_Ignore")
    (bind _astwin_stick_mode (cast `/Game/Blueprints/TwinStickMode` (`GameplayStatics.GetGameMode`)))
    (if (== Player 0)
      (`/Game/Blueprints/TwinStickMode.IncrementScore` _astwin_stick_mode _score)
      (`self.DetachFromControllerPendingDestroy`)
      (`KismetSystemLibrary.Delay` 3.0)
      (`self.K2_DestroyActor`)
      (else
        (`/Game/Blueprints/TwinStickMode.IncrementScore2` _astwin_stick_mode _score)
        (`self.DetachFromControllerPendingDestroy`)
        (`KismetSystemLibrary.Delay` 3.0)
        (`self.K2_DestroyActor`)))))

(event `self.ReceiveActorBeginOverlap`
  (params (OtherActor :type "Actor Object Reference"))
  (bind _ashero_character (cast `/Game/Blueprints/HeroCharacter` OtherActor))
  (set `self.Hero` _ashero_character)
  (`KismetSystemLibrary.K2_SetTimer` null "DamageTheHero" (/ 1.0 (`self.AttackPerSecond`)) true))

(event `DamageTheHero`
  (`/Game/Blueprints/HeroCharacter.AffectHealth` (`self.Hero`) (`self.Damage`) 0))

(event `self.ReceiveActorEndOverlap`
  (params (OtherActor :type "Actor Object Reference"))
  (if (== OtherActor (`self.Hero`))
    (`KismetSystemLibrary.K2_ClearTimer` null "DamageTheHero")))

(fn `UserConstructionScript`
  (`parent.UserConstructionScript`)
  (bind _returnvalue (`PrimitiveComponent.CreateDynamicMaterialInstance` (`self.Mesh`) 0 null))
  (bind _output_get (set `self.DynaMat` _returnvalue))
  (`MaterialInstanceDynamic.SetVectorParameterValue` _output_get "BodyColor" (`self.EnemyColor`)))