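; Projectile actor that deals damage to hostile actors it overlaps.
; On overlap, targets implementing IDamageable without the Friendly tag receive an AffectHealth interface message carrying the damage and owning player.
; Those hits and overlaps with non-damageable actors play a laser sound on the collision component and destroy the projectile.
; Friendly damageable actors are ignored, so the projectile passes through them.
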(event `self.ReceiveActorBeginOverlap`
  (params (OtherActor :type "Actor Object Reference"))
  (if (`KismetSystemLibrary.DoesImplementInterface` OtherActor "/Game/Blueprints/iDamageable.iDamageable_C")
    (if (not (`self.ActorHasTag` OtherActor "Friendly"))
      (message `/Game/Blueprints/iDamageable.AffectHealth` OtherActor (`self.Damage`) (`self.owningPlayer`))
      (`GameplayStatics.SpawnSoundAttached` "/Game/Audio/SoundsCrate-SciFi-Laser5.SoundsCrate-SciFi-Laser5" (`self.Collision`) :!label _label)
      (`self.K2_DestroyActor`))
    (else
      (goto _label))))

(fn `UserConstructionScript`)