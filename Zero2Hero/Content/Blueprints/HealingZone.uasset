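; HealingZone is a temporary area actor that heals hero characters inside its sphere, then destroys itself ten seconds after spawning.
; Sphere overlap assigns an entering hero to one of two slots based on the H1 flag and starts that slot's looping timer.
; Each timer tick adds one health while below 100.
; Leaving the sphere pauses the matching timer and clears its flag.
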(event `self.ReceiveBeginPlay`
  (`KismetSystemLibrary.Delay` 10.0)
  (`self.K2_DestroyActor`))

(event `self.Sphere.OnComponentBeginOverlap`
  (params (OverlappedComponent :type "PrimitiveComponent Object Reference") (OtherActor :type "Actor Object Reference") (OtherComp :type "PrimitiveComponent Object Reference") (OtherBodyIndex :type Integer) (bFromSweep :type Boolean) (SweepResult :type "HitResult Structure (by ref)"))
  (bind _ashero_character (cast `/Game/Blueprints/HeroCharacter` OtherActor))
  (set `self.counter` (+ (`self.counter`) 1))
  (if (`self.h1`)
    (set `self.hero1` _ashero_character)
    (`KismetSystemLibrary.K2_SetTimer` null "heal1" 0.1 true)
    (set `self.h1` true)
    (else
      (set `self.hero2` _ashero_character)
      (`KismetSystemLibrary.K2_SetTimer` null "heal2" 0.1 true)
      (set `self.h2` true))))

(event `self.Sphere.OnComponentEndOverlap`
  (params (OverlappedComponent :type "PrimitiveComponent Object Reference") (OtherActor :type "Actor Object Reference") (OtherComp :type "PrimitiveComponent Object Reference") (OtherBodyIndex :type Integer))
  (bind _ashero_character (cast `/Game/Blueprints/HeroCharacter` OtherActor))
  (if (== _ashero_character (`self.hero1`))
    (`KismetSystemLibrary.K2_PauseTimer` null "heal1")
    (set `self.h1` false)
    (elif (== _ashero_character (`self.hero2`))
      (`KismetSystemLibrary.K2_PauseTimer` null "heal2")
      (set `self.h2` false))))

(fn `heal1`
  (if (< (`/Game/Blueprints/BaseCharacter.Health` (`self.hero1`)) 100.0)
    (`/Game/Blueprints/HeroCharacter.AffectHealth` (`self.hero1`) 1.0 0)))

(fn `heal2`
  (bind _hero2 (`self.hero2`))
  (if (< (`/Game/Blueprints/BaseCharacter.Health` _hero2) 100.0)
    (`/Game/Blueprints/HeroCharacter.AffectHealth` _hero2 1.0 0)))

(fn `UserConstructionScript`)