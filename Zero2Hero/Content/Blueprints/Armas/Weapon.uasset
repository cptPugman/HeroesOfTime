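; Player weapon Blueprint that switches firing behavior on a name string: electric "rayos", shotgun or standard projectile, with "lanzaC" firing nothing here.
; PullTrigger starts a looping Fire timer at the Cadencia rate; ReleaseTrigger clears it.
; The electric mode runs a gated delay loop that sphere-traces ahead, beaming and damaging the first hit actor, or a random cone point on a miss.
; Shotgun sprays randomized pellets; standard shots consume ammo and apply random deviation.
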(event `PullTrigger`
  (params (PlayerID :type Integer))
  (set `self.player ID` PlayerID)
  (`/Engine/EditorBlueprintResources/StandardMacros.DoOnce` false :!label _label
    (:`Completed`
      (`self.Fire`)
      (`KismetSystemLibrary.K2_SetTimer` null "Fire" (/ 1.0 (`self.Cadencia`)) true))))

(event `TargetShot`
  (bind _actorsunderattack (`self.ActorsUnderAttack`))
  (bind _sphere (`self.Sphere`))
  ;[1 1 1] When Targeted to Pawn/Character
  (for (_array_element _array_index) _actorsunderattack
    (if (< _array_index 1)
      (bind _returnvalue (`GameplayStatics.SpawnEmitterAttached` (`self.ParticleMjollnir`) _sphere (`self.Muzzle`) (`SceneComponent.K2_GetComponentLocation` _sphere) (struct) "KeepWorldPosition"))
      (`ParticleSystemComponent.SetBeamTargetPoint` _returnvalue 0 (`self.K2_GetActorLocation` _array_element) 0)
      (bind _asenemy_character (cast `/Game/Blueprints/Enemies/EnemyCharacter` _array_element))
      (`/Game/Blueprints/Enemies/EnemyCharacter.AffectHealth` _asenemy_character -5.0 (`self.player ID`))))
  (`KismetArrayLibrary.Array_Clear` _actorsunderattack))

(event `ReleaseTrigger`
  (bind _returnvalue (+ (`SceneComponent.K2_GetComponentLocation` (`self.SkeletalMesh`)) (* (`SceneComponent.GetForwardVector` (`self.Arrow`)) (`self.spread Radius`))))
  (`KismetSystemLibrary.K2_ClearTimer` null "Fire")
  (if (`KismetStringLibrary.EqualEqual_StrStr` (`self.nombre`) "rayos")
    (`|ExecutionSequence`
      (:`then_0`
        (goto _label_2 :!via `Close`))
      (:`then_1`
        (goto _label :!via `Reset`)))
    (else
      (goto _label :!via `Reset`))))

(event `Fire`
  (bind _nombre (`self.nombre`))
  (bind (_returnvalue_roll _returnvalue_pitch _returnvalue_yaw) (`KismetMathLibrary.BreakRotator` (`KismetMathLibrary.Conv_VectorToRotator` (`SceneComponent.GetForwardVector` (`self.Arrow`)))))
  (bind _returnvalue (+ (`SceneComponent.K2_GetComponentLocation` (`self.SkeletalMesh`)) (* (`SceneComponent.GetForwardVector` (`self.Arrow`)) (`self.spread Radius`))))
  (if (`KismetStringLibrary.EqualEqual_StrStr` _nombre "rayos")
    ;[1 1 1] Electric Weapon
    ;;[1 0 0.9142] Continuous Shooting with firerate by pressing button
    (`|ExecutionSequence`
      (:`then_0`
        (goto _label_2 :!via `Open`))
      (:`then_1`
        (`/Engine/EditorBlueprintResources/StandardMacros.Gate` true :!label _label_2
          (:`Exit`
            (`|ExecutionSequence`
              (:`then_0`
                (bind _outhits (`KismetSystemLibrary.SphereTraceMultiForObjects` _returnvalue (+ _returnvalue (0.0 1.0 0.0)) (`self.spread Radius`) (`self.Objects`) false (`self.actors to ignre`)))
                (for _array_element _outhits
                  (`KismetArrayLibrary.Array_AddUnique` (`self.ActorsUnderAttack`) (`.HitActor` (`GameplayStatics.BreakHitResult` _array_element))))
                (if (> (`KismetArrayLibrary.Array_Length` (`self.actorsUnderAttack`)) 0)
                  (`self.TargetShot`)
                  (else
                    (`self.MissShot`))))
              (:`then_1`
                (`KismetSystemLibrary.Delay` (`self.FireRate`))
                (goto _label_2)))))))
    (elif (`KismetStringLibrary.EqualEqual_StrStr` _nombre "shotgun")
      (for _ (range 11)
        (bind _returnvalue_2 (`|SpawnActorFromClass` "/Game/Blueprints/Armas/Proyectiles/ProjectileShotgun.ProjectileShotgun_C" (`KismetMathLibrary.MakeTransform` (+ (`SceneComponent.K2_GetComponentLocation` (`self.Arrow`)) (`KismetMathLibrary.RandomFloatInRange` -10.0 10.0)) (`KismetMathLibrary.MakeRotator` _returnvalue_roll (+ _returnvalue_pitch (`KismetMathLibrary.RandomFloatInRange` -10.0 10.0)) (+ (`KismetMathLibrary.RandomFloatInRange` -10.0 10.0) _returnvalue_yaw)) (0.2 0.2 0.2)) "Undefined" "OverrideRootScale"))
        (set `/Game/Blueprints/Armas/Proyectiles/Projectile.owningPlayer` (`self.player ID`) _returnvalue_2))
      (elif (`KismetStringLibrary.EqualEqual_StrStr` (`self.nombre`) "lanzaC")
        _
        (elif (> (`self.municion`) 0.0)
          (`GameplayStatics.SpawnSoundAttached` "/Game/Audio/SoundsCrate-SciFi-Laser2.SoundsCrate-SciFi-Laser2" (`self.SkeletalMesh`))
          (if (`self.left`)
            (set `self.Desviacion` (* (`self.Desviacion`) -1.0))
            (set `self.left` false)
            (else
              (set `self.left` true)))
          (bind _returnvalue_3 (`|SpawnActorFromClass` "/Game/Blueprints/Armas/Proyectiles/ProjectileStandard.ProjectileStandard_C" (`SceneComponent.K2_GetComponentToWorld` (`self.Arrow`)) "AlwaysSpawn" "OverrideRootScale"))
          (`/Engine/EditorBlueprintResources/StandardMacros.IsValid` _returnvalue_3
            (:`Is Valid`
              (set `/Game/Blueprints/Armas/Proyectiles/Projectile.desviacion` (* (`KismetMathLibrary.RandomFloat`) (`self.Desviacion`)) _returnvalue_3)
              (set `/Game/Blueprints/Armas/Proyectiles/Projectile.Damage` 100.0 _returnvalue_3))
            (:`Is Not Valid`
              _))
          (set `self.municion` (- (`self.municion`) 1.0))
          (`/Engine/EditorBlueprintResources/StandardMacros.IsValid` _returnvalue_3
            (:`Is Valid`
              (set `/Game/Blueprints/Armas/Proyectiles/Projectile.owningPlayer` (`self.player ID`) _returnvalue_3))))))))

(event `MissShot`
  ;[1 1 1] MissShooting
  (bind (_outhit _returnvalue) (`KismetSystemLibrary.LineTraceSingle` (`SceneComponent.K2_GetComponentLocation` (`self.rayoLase`)) (+ (`SceneComponent.K2_GetComponentLocation` (`self.SkeletalMesh`)) (* (`KismetMathLibrary.RandomUnitVectorInConeWithYawAndPitch` (`SceneComponent.GetForwardVector` (`self.Arrow`)) 60.0 10.0) (`self.spread Radius`))) "TraceTypeQuery1"))
  (bind _returnvalue_2 (`GameplayStatics.SpawnEmitterAttached` (`self.ParticleMjollnir`) (`self.Sphere`) (`self.Muzzle`) (`SceneComponent.K2_GetComponentLocation` (`self.rayoLase`)) (struct) "KeepWorldPosition"))
  (if _returnvalue
    (bind (_bblockinghit _binitialoverlap _time _location _impactpoint _normal _impactnormal _physmat _hitactor _hitcomponent _hitbonename _hititem _faceindex _tracestart _traceend) (`GameplayStatics.BreakHitResult` _outhit))
    (`ParticleSystemComponent.SetBeamTargetPoint` _returnvalue_2 0 _impactpoint 0)
    (else
      (`ParticleSystemComponent.SetBeamTargetPoint` _returnvalue_2 0 _traceend 0))))

(event `self.ReceiveBeginPlay`
  (bind _actors_to_ignre (`self.actors to ignre`))
  (`KismetArrayLibrary.Array_Add` _actors_to_ignre (`GameplayStatics.GetPlayerCharacter` 0))
  (`KismetArrayLibrary.Array_Add` _actors_to_ignre (`GameplayStatics.GetPlayerCharacter` 1))
  (set `self.municion` 1000.0)
  (set `self.Desviacion` 5.0)
  (set `self.Daño` 20.0))

(fn `UserConstructionScript`)