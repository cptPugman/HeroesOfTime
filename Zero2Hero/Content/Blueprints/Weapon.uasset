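; Weapon Blueprint that fires projectiles automatically while the trigger is held.
; PullTrigger fires immediately, then starts a looping timer that calls Fire at the BulletsPerSecond rate, with a DoOnce guarding against repeat pulls.
; Fire plays a laser sound on the skeletal mesh and spawns a Projectile at the Arrow component's world transform.
; ReleaseTrigger clears the timer and resets the DoOnce.
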(event `PullTrigger`
  (`/Engine/EditorBlueprintResources/StandardMacros.DoOnce` false :!label _label
    (:`Completed`
      (`self.Fire`)
      (`KismetSystemLibrary.K2_SetTimer` null "Fire" (/ 1.0 (`self.BulletsPerSecond`)) true))))

(event `ReleaseTrigger`
  (`KismetSystemLibrary.K2_ClearTimer` null "Fire")
  (goto _label :!via `Reset`))

(event `Fire`
  (`GameplayStatics.SpawnSoundAttached` "/Game/Audio/SoundsCrate-SciFi-Laser2.SoundsCrate-SciFi-Laser2" (`self.SkeletalMesh`))
  (`|SpawnActorFromClass` "/Game/Blueprints/Projectile.Projectile_C" (`SceneComponent.K2_GetComponentToWorld` (`self.Arrow`)) "Undefined" "OverrideRootScale"))

(fn `UserConstructionScript`)