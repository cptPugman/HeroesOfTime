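; Shared camera actor for a two-player twin-stick game, set as both controllers' view target on BeginPlay.
; Each tick it centers between the two HeroCharacters and scales spring arm length with their separation, above a minimum.
; It also tethers players by repositioning them around the midpoint, clamped to MaximumDistance.
; When the TwinStickMode game mode flags one player dead, it follows the survivor at fixed arm length.
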(event `self.ReceiveBeginPlay`
  ;[0.7768 0.6133 1] Begin Play : Cambia a la camara a modo multiplayer
  (`PlayerController.SetViewTargetWithBlend` (`GameplayStatics.GetPlayerController` 1) self 0.0 "VTBlend_Linear" 0.0 true)
  (`PlayerController.SetViewTargetWithBlend` (`GameplayStatics.GetPlayerController` 0) self 0.0 "VTBlend_Linear" 0.0 true)
  (bind _outactors (`GameplayStatics.GetAllActorsOfClass` "/Game/Blueprints/HeroCharacter.HeroCharacter_C"))
  (set `self.player1` (`KismetArrayLibrary.Array_Get` _outactors))
  (set `self.player2` (`KismetArrayLibrary.Array_Get` _outactors 1)))

(event `self.ReceiveTick`
  (params (DeltaSeconds :type "Float (single-precision)"))
  (bind _returnvalue (`self.K2_GetActorLocation`))
  (bind _distance (`self.distance`))
  (bind _springarm (`self.SpringArm`))
  (bind _returnvalue_2 (`KismetMathLibrary.VSize` _distance))
  (bind _returnvalue_3 (/ (`KismetMathLibrary.ClampVectorSize` (`self.distance`) 0.0 (`self.maximum distance`)) 2))
  ;[0.7559 1 0.7958] Manejo de la Cámara : Actualmente 3 opciones : Ambos jugadores Vivos , Jugador 1 Muerto , Jugador 2 Muerto
  ;;[0 1 0.2413] TICK
  (set `self.position` (`self.K2_GetActorLocation` self))
  ;;[0.2327 1 0.3823] Jugador 1 Muerto , Caámara sigue al Jugador 2
  (bind _astwin_stick_mode (cast `/Game/Blueprints/TwinStickMode` (`GameplayStatics.GetGameMode`)))
  (if (`/Game/Blueprints/TwinStickMode.player1Dead` _astwin_stick_mode)
    (if (not (`/Game/Blueprints/TwinStickMode.player2Dead` _astwin_stick_mode))
      (bind _ashero_character (cast `/Game/Blueprints/HeroCharacter` (`GameplayStatics.GetPlayerCharacter` 1)))
      (`self.K2_SetActorLocation` self (`self.K2_GetActorLocation` _ashero_character) true false)
      (set `SpringArmComponent.TargetArmLength` 500.0 (`self.SpringArm`)))
    (else
      ;;[0.333 1 0.5702] Jugador 2 Muerto, Cámara sigue a jugador 1
      (if (`/Game/Blueprints/TwinStickMode.player2Dead` _astwin_stick_mode)
        (if (not (`/Game/Blueprints/TwinStickMode.player1Dead` _astwin_stick_mode))
          (bind _ashero_character_2 (cast `/Game/Blueprints/HeroCharacter` (`GameplayStatics.GetPlayerCharacter` 0)))
          (`self.K2_SetActorLocation` self (`self.K2_GetActorLocation` _ashero_character_2) true false)
          (set `SpringArmComponent.TargetArmLength` 500.0 (`self.SpringArm`)))
        (else
          ;;[0.3591 1 0.5123] Ambos Jugadores Vivos, Cámara en medio de los 2
          (bind _outactors (`GameplayStatics.GetAllActorsOfClass` "/Game/Blueprints/HeroCharacter.HeroCharacter_C"))
          (set `self.player1` (`KismetArrayLibrary.Array_Get` _outactors))
          (set `self.player2` (`KismetArrayLibrary.Array_Get` _outactors 1))
          (set `self.distance` (- (`self.K2_GetActorLocation` (`self.player1`)) (`self.K2_GetActorLocation` (`self.player2`))))
          (`|ExecutionSequence`
            (:`then_0`
              (`self.K2_SetActorLocation` (+ (`self.K2_GetActorLocation` (`self.player2`)) (/ _distance 2)))
              (if (< _returnvalue_2 500.0)
                (set `SpringArmComponent.TargetArmLength` 500.0 _springarm)
                (else
                  (set `SpringArmComponent.TargetArmLength` _returnvalue_2 _springarm))))
            (:`then_1`
              (`self.K2_SetActorLocation` (`self.player1`) (+ _returnvalue _returnvalue_3) false false)
              (`self.K2_SetActorLocation` (`self.player2`) (- _returnvalue _returnvalue_3) false false))))))))

(fn `UserConstructionScript`)