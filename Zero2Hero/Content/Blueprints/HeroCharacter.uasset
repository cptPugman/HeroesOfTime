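; Player hero character for a twin-stick shooter, with axis-driven movement, aim-to-fire shooting and taunt states.
; BeginPlay attaches a spawned weapon to the gun socket, stores the spawn transform in TwinStickMode and adds the HUD.
; Look input past a deadzone sets control rotation and pulls the trigger, tagged by player; movement cancels taunts.
; On death, input stops, then after a delay GameMode respawns the player and character and weapon are destroyed.
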(event `self.ReceiveBeginPlay`
  (bind _mesh (`self.Mesh`))
  (if (== (`self.GetController`) (`GameplayStatics.GetPlayerController` 0))
    (`self.K2_AddActorLocalOffset` (0.0 200.0 0.0)))
  (`|ExecutionSequence`
    (:`then_0`
      (bind _returnvalue (`|SpawnActorFromClass` "/Game/Blueprints/Weapon.Weapon_C" (`SceneComponent.K2_GetComponentToWorld` _mesh) "Undefined" "OverrideRootScale"))
      (bind _output_get (set `self.Weapon` _returnvalue))
      (`self.K2_AttachRootComponentTo` _output_get _mesh "GunSocket" "SnapToTarget" true))
    (:`then_1`
      (bind _astwin_stick_mode (cast `/Game/Blueprints/TwinStickMode` (`GameplayStatics.GetGameMode`)))
      (bind _output_get_2 (set `self.GameMode` _astwin_stick_mode))
      (set `/Game/Blueprints/TwinStickMode.PlayerSpawnTransform` (`self.GetTransform`) _output_get_2))
    (:`then_2`
      (bind _returnvalue_2 (`|CreateWidget` "/Game/Blueprints/TwinStickHUD.TwinStickHUD_C"))
      (`UserWidget.AddToViewport` _returnvalue_2 0))))

(event `InputAxis|MoveUp`
  (params (AxisValue :type "Float (single-precision)"))
  ;[1 1 1] Movement
  (`self.AddMovementInput` (1.0 0.0 0.0) AxisValue))

(event `InputAxis|LookUp`
  (params (AxisValue :type "Float (single-precision)"))
  (bind _weapon (`self.Weapon`))
  ;[1 1 1] Rotation
  (bind _returnvalue (`KismetMathLibrary.MakeVector` AxisValue (stale `InputAxis|LookRight` AxisValue)))
  (if (> (`KismetMathLibrary.VSize` _returnvalue) 0.25) :!label _label
    (`Controller.SetControlRotation` (`self.GetController`) (`KismetMathLibrary.Conv_VectorToRotator` _returnvalue))
    ;[1 0.365 0.365] Para Saber Quien dispara
    (if (== (`self.GetController`) (`GameplayStatics.GetPlayerController` 0))
      (`/Game/Blueprints/Weapon.PullTrigger` _weapon 0)
      (else
        (`/Game/Blueprints/Weapon.PullTrigger` _weapon 1)))
    (else
      (`/Game/Blueprints/Weapon.ReleaseTrigger` _weapon))))

(event `InputAxis|LookRight`
  (params (AxisValue :type "Float (single-precision)"))
  ;[1 1 1] Rotation
  (goto _label))

(event `InputAxis|MoveRight`
  (params (AxisValue :type "Float (single-precision)"))
  ;[1 1 1] Movement
  (`self.AddMovementInput` (0.0 1.0 0.0) AxisValue))

(event `/Game/Blueprints/iDamageable.AffectHealth`
  (params (Delta :type "Float (single-precision)") (Player :type Integer))
  (`self.CalculateHealth` Delta)
  (if (`self.IsDead`)
    (`self.DisableInput` null)
    (`/Game/Blueprints/Weapon.ReleaseTrigger` (`self.Weapon`))
    (`KismetSystemLibrary.Delay` 3.0)
    ;[1 1 1] Modificado 08/03
    (`/Game/Blueprints/TwinStickMode.RespawnPlayer` (`self.GameMode`) (`self.GetController`))
    (`self.K2_DestroyActor` (`self.Weapon`))
    (`self.K2_DestroyActor` self)
    (bind _outactors (`GameplayStatics.GetAllActorsOfClass` "/Game/Blueprints/Camera.Camera_C"))
    (`PlayerController.SetViewTargetWithBlend` (`GameplayStatics.GetPlayerController` 0) (`KismetArrayLibrary.Array_Get` _outactors) 0.0 "VTBlend_Linear" 0.0 false)))

(event `InputAction|Taunts`
  (params (Key :type "Key Structure" :default "AnyKey"))
  (:`Pressed`
    (set `self.taunts` true))
  (:`Released`
    (set `self.taunts` false)))

(event `InputAction|Taunt_Dance`
  (params (Key :type "Key Structure" :default "AnyKey"))
  (:`Pressed`
    (set `self.dancing` true)
    (set `self.taunting` false)
    (set `self.laughing` false)
    (set `self.standing` false)))

(event `InputAction|Taunt_StandUp`
  (params (Key :type "Key Structure" :default "AnyKey"))
  (:`Pressed`
    (set `self.standing` true)
    (set `self.taunting` false)
    (set `self.dancing` false)
    (set `self.laughing` false)))

(event `InputAction|Taunt_Laugh`
  (params (Key :type "Key Structure" :default "AnyKey"))
  (:`Pressed`
    (set `self.laughing` true)
    (set `self.taunting` false)
    (set `self.dancing` false)
    (set `self.standing` false)))

(event `InputAction|Taunt_Taunt`
  (params (Key :type "Key Structure" :default "AnyKey"))
  (:`Pressed`
    (set `self.taunting` true)
    (set `self.dancing` false)
    (set `self.laughing` false)
    (set `self.standing` false)))

(event `self.ReceiveTick`
  (params (DeltaSeconds :type "Float (single-precision)"))
  (bind _returnvalue (`KismetMathLibrary.VSize` (`CharacterMovementComponent.GetCurrentAcceleration` (`self.CharacterMovement`))))
  (if (> _returnvalue 0.0)
    (set `self.NewVar_0` _returnvalue)
    (if (or (`self.taunting`) (`self.laughing`) (`self.standing`) (`self.dancing`))
      (set `self.taunting` false)
      (set `self.dancing` false)
      (set `self.laughing` false)
      (set `self.standing` false))))

(fn `UserConstructionScript`
  (`parent.UserConstructionScript`))