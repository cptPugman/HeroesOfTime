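; Round manager that runs escalating waves of AI EnemyCharacters.
; A looping timer calls spawnEnemies, which fills up to four cached TargetPoints in turn while under the concurrent cap and the round's remaining budget.
; An exhausted budget triggers StartRound through a DoOnce, even with enemies still alive; after a delay it advances the round and scales budget and cap.
; Tick sets EnemiesAlive to unspawned plus live enemies.
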(event `self.ReceiveBeginPlay`
  (bind _outactors (`GameplayStatics.GetAllActorsOfClass` "/Script/Engine.TargetPoint"))
  (set `self.Point1` (`KismetArrayLibrary.Array_Get` _outactors))
  (set `self.Point2` (`KismetArrayLibrary.Array_Get` _outactors 1))
  (set `self.Point3` (`KismetArrayLibrary.Array_Get` _outactors 2))
  (set `self.Point4` (`KismetArrayLibrary.Array_Get` _outactors 3))
  (`KismetSystemLibrary.K2_SetTimer` null "spawnEnemies" 5.0 true))

(event `StartRound`
  (`KismetSystemLibrary.Delay` 10.0)
  (set `self.RoundNumber` (+ (`self.RoundNumber`) 1))
  (bind _output_get (set `self.MaxEnemiesVariable` (* (`self.maxEnemies`) 1.4)))
  (set `self.maxEnemies` _output_get)
  (set `self.ConcurrentEnemies` (`KismetMathLibrary.FTrunc` (* (`self.ConcurrentEnemies`) 1.4))))

(event `self.ReceiveTick`
  (params (DeltaSeconds :type "Float (single-precision)"))
  (bind _outactors (`GameplayStatics.GetAllActorsOfClass` "/Game/Blueprints/EnemyCharacter.EnemyCharacter_C"))
  (set `self.enemiesAlive` (+ (`self.MaxEnemiesVariable`) (`KismetMathLibrary.Conv_IntToDouble` (`KismetArrayLibrary.Array_Length` _outactors)))))

(fn `spawnEnemies`
  (bind _outactors (`GameplayStatics.GetAllActorsOfClass` "/Game/Blueprints/EnemyCharacter.EnemyCharacter_C"))
  (if (and (< (`KismetArrayLibrary.Array_Length` _outactors) (`self.ConcurrentEnemies`)) (> (`self.MaxEnemiesVariable`) 0.0))
    (`AIBlueprintHelperLibrary.SpawnAIFromClass` "/Game/Blueprints/EnemyCharacter.EnemyCharacter_C" null (`self.K2_GetActorLocation` (`self.Point1`)))
    (set `self.MaxEnemiesVariable` (- (`self.MaxEnemiesVariable`) 1.0))
    (bind _outactors_2 (`GameplayStatics.GetAllActorsOfClass` "/Game/Blueprints/EnemyCharacter.EnemyCharacter_C"))
    (if (and (< (`KismetArrayLibrary.Array_Length` _outactors_2) (`self.ConcurrentEnemies`)) (> (`self.MaxEnemiesVariable`) 0.0))
      (`AIBlueprintHelperLibrary.SpawnAIFromClass` "/Game/Blueprints/EnemyCharacter.EnemyCharacter_C" null (`self.K2_GetActorLocation` (`self.Point2`)))
      (set `self.MaxEnemiesVariable` (- (`self.MaxEnemiesVariable`) 1.0))
      (bind _outactors_3 (`GameplayStatics.GetAllActorsOfClass` "/Game/Blueprints/EnemyCharacter.EnemyCharacter_C"))
      (if (and (< (`KismetArrayLibrary.Array_Length` _outactors_3) (`self.ConcurrentEnemies`)) (> (`self.MaxEnemiesVariable`) 0.0))
        (`AIBlueprintHelperLibrary.SpawnAIFromClass` "/Game/Blueprints/EnemyCharacter.EnemyCharacter_C" null (`self.K2_GetActorLocation` (`self.Point3`)))
        (set `self.MaxEnemiesVariable` (- (`self.MaxEnemiesVariable`) 1.0))
        (bind _outactors_4 (`GameplayStatics.GetAllActorsOfClass` "/Game/Blueprints/EnemyCharacter.EnemyCharacter_C"))
        (if (and (< (`KismetArrayLibrary.Array_Length` _outactors_4) (`self.ConcurrentEnemies`)) (> (`self.MaxEnemiesVariable`) 0.0))
          (`AIBlueprintHelperLibrary.SpawnAIFromClass` "/Game/Blueprints/EnemyCharacter.EnemyCharacter_C" null (`self.K2_GetActorLocation` (`self.Point4`)))
          (set `self.MaxEnemiesVariable` (- (`self.MaxEnemiesVariable`) 1.0))))))
  (if (<= (`self.MaxEnemiesVariable`) 0.0)
    (`/Engine/EditorBlueprintResources/StandardMacros.DoOnce` false :!label _label
      (:`Completed`
        (`self.StartRound`)))
    (else
      (goto _label :!via `Reset`))))

(fn `UserConstructionScript`)