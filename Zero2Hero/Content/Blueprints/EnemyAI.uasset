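; Enemy AI controller Blueprint that makes its pawn chase the nearer of two HeroCharacter players.
; A looping timer started on BeginPlay calls TrackPlayer every second, which compares distances to players 0 and 1 and issues AIMoveTo.
; If the nearer hero is dead, it targets the other without checking that one's death state.
; When only one hero exists, it follows that hero regardless of death.
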(event `self.ReceiveBeginPlay`
  (`KismetSystemLibrary.K2_SetTimer` null "TrackPlayer" 1.0 true))

(event `TrackPlayer`
  (bind _returnvalue (`GameplayStatics.GetPlayerCharacter` 1))
  (bind _returnvalue_2 (`GameplayStatics.GetPlayerCharacter` 0))
  (bind _returnvalue_3 (`self.K2_GetActorLocation` (`self.K2_GetPawn`)))
  ;[1 1 1] Mira que jugador esta mas cerca y lo persigue
  (cast `/Game/Blueprints/HeroCharacter` (`GameplayStatics.GetPlayerCharacter` 1)
    (:`then`
      (cast `/Game/Blueprints/HeroCharacter` (`GameplayStatics.GetPlayerCharacter` 0)
        (:`then`
          (if (< (`KismetMathLibrary.VSize` (- (`self.K2_GetActorLocation` _returnvalue_2) _returnvalue_3)) (`KismetMathLibrary.VSize` (- (`self.K2_GetActorLocation` _returnvalue) _returnvalue_3)))
            (bind _ashero_character (cast `/Game/Blueprints/HeroCharacter` _returnvalue_2 :!label _label)
              (:`then`
                (if (`/Game/Blueprints/BaseCharacter.IsDead` _ashero_character)
                  (`|AIMoveTo` (`self.K2_GetPawn`) (0.0 0.0 0.0) _returnvalue :!label _label_2)
                  (else
                    (`|AIMoveTo` (`self.K2_GetPawn`) (0.0 0.0 0.0) _returnvalue_2 :!label _label_3))))
              (:`CastFailed`
                (bind _ashero_character_2 (cast `/Game/Blueprints/HeroCharacter` _returnvalue :!label _label_4)
                  (:`then`
                    (if (`/Game/Blueprints/BaseCharacter.IsDead` _ashero_character_2)
                      (goto _label_3)
                      (else
                        (goto _label_2))))
                  (:`CastFailed`
                    (goto _label)))))
            (else
              (goto _label_4))))
        (:`CastFailed`
          (bind _ashero_character_3 (cast `/Game/Blueprints/HeroCharacter` (`GameplayStatics.GetPlayerCharacter` 1)))
          (`|AIMoveTo` (`self.K2_GetPawn`) (0.0 0.0 0.0) _ashero_character_3))))
    (:`CastFailed`
      (bind _ashero_character_4 (cast `/Game/Blueprints/HeroCharacter` (`GameplayStatics.GetPlayerCharacter` 0)))
      (`|AIMoveTo` (`self.K2_GetPawn`) (0.0 0.0 0.0) _ashero_character_4))))

(fn `UserConstructionScript`)