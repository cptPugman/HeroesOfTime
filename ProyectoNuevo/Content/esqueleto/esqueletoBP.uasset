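; Skeleton enemy that plays a running animation, climbs ladders and is destroyed when hit by an arrow.
; Tick polls all TriggerVolumes: an "escalera" overlap starts climbing by raising its location each frame.
; A "top" overlap plays a timed climb-over with a forward push, then loops a punching animation.
; A repeating timer polls Arrow overlaps, and construction attaches both fist components to hand sockets.
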(event `self.ReceiveBeginPlay`
  (`SkeletalMeshComponent.PlayAnimation` (`self.Mesh`) "/Game/esqueleto/animations/running_inPlace_mixamo_com.running_inPlace_mixamo_com" true)
  (`KismetSystemLibrary.K2_SetTimer` null "detectaArrow" 0.1 true))

(event `self.ReceiveTick`
  (params (DeltaSeconds :type "Float (single-precision)"))
  (bind _returnvalue (`self.K2_GetActorLocation` self))
  (if (`self.escalando`)
    (if (`self.top`)
      (set `self.newLocation` (+ (`self.newLocation`) (* (`self.GetActorForwardVector` self) 1)))
      (else
        (bind _output_get (set `self.newLocation` (+ (`self.newLocation`) (0.0 0.0 1.8))))))
    (`self.K2_SetActorLocation` self _output_get false false)
    (bind _outactors (`GameplayStatics.GetAllActorsOfClass` "/Script/Engine.TriggerVolume"))
    (for _array_element _outactors
      (if (`PrimitiveComponent.IsOverlappingActor` (`self.Mesh`) _array_element)
        (if (`self.ActorHasTag` _array_element "top")
          (`/Engine/EditorBlueprintResources/StandardMacros.DoOnce` false
            (:`Completed`
              (`SkeletalMeshComponent.PlayAnimation` (`self.Mesh`) "/Game/esqueleto/animations/climbing_mixamo_com.climbing_mixamo_com" false)
              (`KismetSystemLibrary.Delay` 2.47)
              (set `self.top` true)
              (`KismetSystemLibrary.Delay` 1.36)
              (`SkeletalMeshComponent.PlayAnimation` (`self.Mesh`) "/Game/esqueleto/animations/zombie_punching__1__mixamo_com.zombie_punching__1__mixamo_com" true)
              (set `self.escalando` false))))))
    (else
      (bind _outactors_2 (`GameplayStatics.GetAllActorsOfClass` "/Script/Engine.TriggerVolume"))
      (for _array_element_2 _outactors_2
        (if (`PrimitiveComponent.IsOverlappingActor` (`self.Mesh`) _array_element_2)
          (if (`self.ActorHasTag` _array_element_2 "escalera")
            (set `self.escalando` true)
            (`self.K2_SetActorLocation` self _returnvalue false false)
            (set `self.newLocation` _returnvalue)
            (`SkeletalMeshComponent.PlayAnimation` (`self.Mesh`) "/Game/esqueleto/animations/climbing_up_wall_mixamo_com.climbing_up_wall_mixamo_com" true)))))))

(fn `detectaArrow`
  (bind _outactors (`GameplayStatics.GetAllActorsOfClass` "/Game/Blueprints/Weapons/Arrow.Arrow_C"))
  (for _array_element _outactors
    (if (`self.IsOverlappingActor` _array_element self)
      (`self.K2_DestroyActor` self))))

(fn `UserConstructionScript`
  (bind _mesh (`self.Mesh`))
  (`SceneComponent.K2_AttachTo` (`self.puño derecho`) _mesh "RightHandIndex1" "SnapToTargetIncludingScale" true)
  (`SceneComponent.K2_AttachTo` (`self.puño izquierdo`) _mesh "LeftHandIndex1" "SnapToTargetIncludingScale" true))