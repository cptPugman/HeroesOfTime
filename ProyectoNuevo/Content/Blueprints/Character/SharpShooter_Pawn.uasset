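; VR player pawn for a sharpshooter game, using floor-level tracking and motion-controller hands.
; On BeginPlay it caches the left and right hand Blueprints from child actors and links each to the other.
; Grip presses and releases call Grab and Release on the matching hand.
; A looping timer calls Teleport every five seconds, cycling the pawn through four preset locations without sweeping.
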(event `self.ReceiveBeginPlay`
  (`KismetSystemLibrary.PrintString` "Hello")
  (`HeadMountedDisplayFunctionLibrary.SetTrackingOrigin` "Floor")
  (`self.RegisterHandBPs`)
  (`KismetSystemLibrary.K2_SetTimer` null "teleport" 5.0 true))

(event `Key|MotionController_Left_Grip1`
  (params (Key :type "Key Structure" :default "AnyKey"))
  (bind _lefthandbp (`self.LeftHandBP`))
  (:`Pressed`
    (`/Game/Blueprints/Character/Hands/BP_LeftHand.Grab` _lefthandbp))
  (:`Released`
    (`/Game/Blueprints/Character/Hands/BP_LeftHand.Release` _lefthandbp)))

(event `Key|MotionController_Right_Grip1`
  (params (Key :type "Key Structure" :default "AnyKey"))
  (bind _righthandbp (`self.RightHandBP`))
  (:`Pressed`
    (`/Game/Blueprints/Character/Hands/BP_LeftHand.Grab` _righthandbp))
  (:`Released`
    (`/Game/Blueprints/Character/Hands/BP_LeftHand.Release` _righthandbp)))

(fn `RegisterHandBPs`
  (bind _lefthandbp (`self.LeftHandBP`))
  (bind _asbp_left_hand (cast `/Game/Blueprints/Character/Hands/BP_LeftHand` (`ChildActorComponent.ChildActor` (`self.LHandChildActor`))))
  (set `self.LeftHandBP` _asbp_left_hand)
  (bind _asbp_right_hand (cast `/Game/Blueprints/Character/Hands/BP_RightHand` (`ChildActorComponent.ChildActor` (`self.RHandChildActor`))))
  (bind _output_get (set `self.RightHandBP` _asbp_right_hand))
  (set `/Game/Blueprints/Character/Hands/BP_LeftHand.OtherHandBlueprint` _output_get _lefthandbp)
  (set `/Game/Blueprints/Character/Hands/BP_LeftHand.OtherHandBlueprint` _lefthandbp (`self.RightHandBP`)))

(fn `teleport`
  (if (== (`self.posicion`) 4)
    (`self.K2_SetActorLocation` self (`self.location1`) false true)
    (set `self.posicion` 1)
    (elif (== (`self.posicion`) 1)
      (`self.K2_SetActorLocation` self (`self.location2`) false true)
      (set `self.posicion` 2)
      (elif (== (`self.posicion`) 2)
        (`self.K2_SetActorLocation` self (`self.location3`) false true)
        (set `self.posicion` 3)
        (elif (== (`self.posicion`) 3)
          (`self.K2_SetActorLocation` self (`self.location4`) false true)
          (set `self.posicion` 4))))))

(fn `UserConstructionScript`)