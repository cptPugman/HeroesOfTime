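; Blueprint interface that lets objects respond to interaction from a player's hands, apparently motion-controller hands in VR.
; It declares pressed and released calls for grab and trigger, plus hand overlap begin and end, each identifying which hand acts.
; Press and overlap-begin calls also receive the hand Blueprint.
; Both press calls report item pickup, secondary grab and a local grab location, while the other calls return a single value.
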(fn `GrabPressed*`
  (params (WhichHand :type "/Game/Blueprints/Enums/LeftRight Enum") (HandBP :type "/Game/Blueprints/Character/Hands/BP_LeftHand Object Reference"))
  (returns (GrabTransform :type "Transform Structure") (ItemPickedUp :type Boolean) (SecondaryGrab :type Boolean) (LocalGrabLocation :type "Vector Structure"))
  (return (struct) false false (0.0 0.0 0.0)))

(fn `GrabReleased*`
  (params (WhichHand :type "/Game/Blueprints/Enums/LeftRight Enum"))
  (returns (`DropOnRelase?` :type Boolean))
  (return false))

(fn `HandBeginOverlap*`
  (params (WhichHand :type "/Game/Blueprints/Enums/LeftRight Enum") (HandBP :type "/Game/Blueprints/Character/Hands/BP_LeftHand Object Reference"))
  (returns (Reply :type Boolean) (SelectionMID :type "MaterialInstanceDynamic Object Reference"))
  (return false null))

(fn `HandEndOverlap*`
  (params (WhichHand :type "/Game/Blueprints/Enums/LeftRight Enum"))
  (returns (NewParam :type Boolean))
  (return false))

(fn `TriggerPressed*`
  (params (WhichHand :type "/Game/Blueprints/Enums/LeftRight Enum") (HandBP :type "/Game/Blueprints/Character/Hands/BP_LeftHand Object Reference"))
  (returns (GrabTransform :type "Transform Structure") (ItemPickedUp :type Boolean) (SecondaryGrab :type Boolean) (LocalGrabLoction :type "Vector Structure"))
  (return (struct) false false (0.0 0.0 0.0)))

(fn `TriggerReleased*`
  (params (WhichHand :type "/Game/Blueprints/Enums/LeftRight Enum"))
  (returns (`DropOnRelease?` :type Boolean))
  (return false))