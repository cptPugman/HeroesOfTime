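; Punchman is an X-Bot enemy pawn that wanders and is destroyed when QuitarVida drains its health (Vida).
; Each tick it randomly nudges a heading angle and applies a local offset from it, converting to radians despite using degree-based trig.
; Construction snaps both hand components to the Enemy's hand sockets.
; Player chasing, close-range punch state, AIMoveTo and overlap logic are present but disconnected, so they never run.
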(event `self.ReceiveTick`
  (params (DeltaSeconds :type "Float (single-precision)"))
  (bind _angle (`self.angle`))
  (bind _output_get (set `self.angleDelta` (* (`self.wanderMaxChange`) (`KismetMathLibrary.RandomFloatInRange` -25.0 25.0))))
  (bind _output_get_2 (set `self.angle` (`KismetMathLibrary.Lerp` _angle (+ _angle _output_get) 0.8)))
  (bind _output_get_3 (set `self.speed` (`KismetMathLibrary.MakeVector` (* (`KismetMathLibrary.DegCos` (* _output_get_2 (/ (`KismetMathLibrary.GetPI`) 180.0))) (`self.K_MAX_SPEED`) 0.8) (* (`KismetMathLibrary.DegSin` (* _output_get_2 (/ (`KismetMathLibrary.GetPI`) 180.0))) (`self.K_MAX_SPEED`) 0.8))))
  (`self.K2_AddActorLocalOffset` (/ _output_get_3 100.0))
  (set `self.angleDelta` 0.0))

(fn `quitarVida`
  (params (hit :type Integer))
  (bind _vida (`self.Vida`))
  (set `self.Vida` (- _vida hit))
  (if (<= _vida 0)
    (`self.K2_DestroyActor`)))

(fn `UserConstructionScript`
  (bind _enemy (`self.Enemy`))
  (`SceneComponent.K2_AttachToComponent` (`self.manoIzquierda`) _enemy "LeftHand" "SnapToTarget" "SnapToTarget" "SnapToTarget" true)
  (`SceneComponent.K2_AttachToComponent` (`self.manoDerecha`) _enemy "RightHand" "SnapToTarget" "SnapToTarget" "SnapToTarget" true))