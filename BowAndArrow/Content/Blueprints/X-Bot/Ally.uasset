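; Ally pawn that hunts and punches the nearest zombie, and destroys itself when its Vida health runs out.
; Every Tick it queries ZombiesManager for the nearest target, seeded by each Punchman actor, turns the YBot mesh toward it and uses AIMoveTo to approach.
; In close range it stops and sets Puncherino; right-hand overlap deals damage through a DoOnce that resets when overlap ends.
; Construction snaps both hand components to YBot sockets.
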(event `self.ReceiveTick`
  (params (DeltaSeconds :type "Float (single-precision)"))
  (bind _y_bot (`self.Y_Bot`))
  (bind _floatingpawnmovement (`self.FloatingPawnMovement`))
  (bind _returnvalue (`SceneComponent.K2_GetComponentLocation` _y_bot))
  (set `FloatingPawnMovement.MaxSpeed` 500.0 _floatingpawnmovement)
  (bind _outactors (`GameplayStatics.GetAllActorsOfClass` "/Game/ZombiesManager/ZombiesManager.ZombiesManager_C"))
  (for _array_element _outactors
    _)
  (bind _outactors_2 (`GameplayStatics.GetAllActorsOfClass` "/Game/X-Bot/Punchman.Punchman_C"))
  (for _array_element_2 _outactors_2
    (bind (_nearestzombie _valid_) (`/Game/ZombiesManager/ZombiesManager.getNearest` _array_element _returnvalue _array_element_2))
    (if _valid_
      (bind _returnvalue_2 (`self.K2_GetActorLocation` _nearestzombie))
      (`KismetSystemLibrary.PrintString` (`KismetStringLibrary.Conv_DoubleToString` (`KismetMathLibrary.VSize` (- _returnvalue_2 _returnvalue))))
      (bind _returnvalue_3 (`self.K2_GetActorLocation` _nearestzombie))
      (`SceneComponent.K2_SetRelativeRotation` _y_bot (`KismetMathLibrary.MakeRotator` (.roll (`SceneComponent.RelativeRotation` _y_bot)) (.pitch (`SceneComponent.RelativeRotation` _y_bot)) (+ (.yaw (`KismetMathLibrary.FindLookAtRotation` _returnvalue _returnvalue_3)) -80.0)) false false)
      (if (< (`KismetMathLibrary.VSize` (- _returnvalue _returnvalue_2)) 140.0)
        (`MovementComponent.StopMovementImmediately` _floatingpawnmovement)
        (set `self.puncherino` true)
        (if (`PrimitiveComponent.IsOverlappingActor` (`self.manoDerecha`) _nearestzombie)
          (`/Engine/EditorBlueprintResources/StandardMacros.DoOnce` false :!label _label
            (:`Completed`
              (`/Game/X-Bot/Punchman.quitarVida` _nearestzombie 50)))
          (else
            (goto _label :!via `Reset`)))
        (else
          (set `self.puncherino` false)
          (`|AIMoveTo` _floatingpawnmovement self _returnvalue_3 null 5.0))))))

(fn `quitarVida`
  (params (hit :type Integer))
  (bind _vida (`self.Vida`))
  (set `self.Vida` (- _vida hit))
  (if (<= _vida 0)
    (`self.K2_DestroyActor`)))

(fn `UserConstructionScript`
  (bind _y_bot (`self.Y_Bot`))
  (`SceneComponent.K2_AttachToComponent` (`self.manoIzquierda`) _y_bot "LeftHand" "SnapToTarget" "SnapToTarget" "SnapToTarget" true)
  (`SceneComponent.K2_AttachToComponent` (`self.manoDerecha`) _y_bot "RightHand" "SnapToTarget" "SnapToTarget" "SnapToTarget" true))