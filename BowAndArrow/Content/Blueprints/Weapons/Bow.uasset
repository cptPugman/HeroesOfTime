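; Two-handed motion-controller bow: one hand holds it, the other pulls the string to nock and fire arrows.
; While pulled, Tick aims the arrow through the holding side's nook, deforms the string via material parameters and drives haptics from draw change.
; Release launches the arrow at a speed scaling with clamped draw length squared, and a spring solve settles the string.
; An optional triple-shot bonus handles two extra angled arrows.
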(event `self.ReceiveTick`
  (params (DeltaSeconds :type "Float (single-precision)"))
  (bind _returnvalue (`GameplayStatics.GetPlayerController` 0))
  (bind _stringmid (`self.StringMID`))
  (bind _returnvalue_2 (- (`SceneComponent.K2_GetComponentLocation` (select `/Game/Blueprints/Enums/LeftRight` (`self.HoldingHand`) :`NewEnumerator0` (`self.LSideNook`) :`NewEnumerator1` (`self.RSideNook`))) (`self.CurrentGrabSpot`)))
  (if (`self.PullingString?`)
    ;[1 1 1] Pull String
    (bind _output_get (set `self.CurrentGrabSpot` (+ (`SceneComponent.K2_GetComponentLocation` (`/Game/Blueprints/Character/Hands/BP_LeftHand.Scene` (`self.StringHandBP`))) (`self.InitialStringGrabOffset`))))
    (`MaterialInstanceDynamic.SetScalarParameterValue` _stringmid "Grabbed" 1.0)
    (`MaterialInstanceDynamic.SetVectorParameterValue` _stringmid "GrabSpot" (`KismetMathLibrary.Conv_VectorToLinearColor` _output_get))
    (set `self.Length` (`KismetMathLibrary.VSize` (- (`SceneComponent.K2_GetComponentLocation` (`self.StringSphere`)) (`self.CurrentGrabSpot`))))
    (`self.K2_SetActorTransform` (`KismetMathLibrary.MakeTransform` (+ (`self.CurrentGrabSpot`) (* (`KismetMathLibrary.Normal` _returnvalue_2) 30.0)) (`KismetMathLibrary.MakeRotFromX` _returnvalue_2)))
    (`self.UpdateBonusArrows`)
    (`self.Haptics/Force Feedback`)
    (else
      ;[1 1 1] String Tension
      (bind _new_p (`/Game/Blueprints/Libraries/PhysicsMacros.SpringSolve` (`self.CurrentGrabSpot`) (`SceneComponent.K2_GetComponentLocation` (`self.StringMesh`)) 0.5 40.0 (`GameplayStatics.GetWorldDeltaSeconds`))
        (:`OUT`
          (`MaterialInstanceDynamic.SetVectorParameterValue` (`self.StringMID`) "GrabSpot" (`KismetMathLibrary.Conv_VectorToLinearColor` _new_p))
          (set `self.CurrentGrabSpot` _new_p)
          (`PlayerController.SetHapticsByValue` _returnvalue 0.0 0.0 (select `/Game/Blueprints/Enums/LeftRight` (`self.StringPullHand`) :`NewEnumerator0` "Left" :`NewEnumerator1` "Right" :!type "EControllerHand Enum"))
          (`PlayerController.ClientPlayForceFeedback` _returnvalue "/Game/Blueprints/ViveForces/Force_Right_0.Force_Right_0" false "None"))))))

(fn `FireBonusArrows`
  (bind _projectilemovement (`self.ProjectileMovement`))
  (bind _projectilemovement_2 (`self.ProjectileMovement`))
  (bind _returnvalue (* (`KismetMathLibrary.FClamp` (`self.Length`) 0.0 35.0) 2.0))
  (bind _returnvalue_2 (`KismetMathLibrary.MakeVector` (* (* _returnvalue _returnvalue) 1.0)))
  (`/Engine/EditorBlueprintResources/StandardMacros.IsValid` null
    (:`Is Valid`
      (`ActorComponent.SetActive` _projectilemovement_2 true false)
      (`ProjectileMovementComponent.SetVelocityInLocalSpace` _projectilemovement_2 _returnvalue_2)
      (set `ProjectileMovementComponent.bRotationFollowsVelocity` true _projectilemovement_2)
      (set `self.BonusArrow1` null))
    (:`Is Not Valid`
      _))
  (`/Engine/EditorBlueprintResources/StandardMacros.IsValid` null
    (:`Is Valid`
      (`ActorComponent.SetActive` _projectilemovement true false)
      (`ProjectileMovementComponent.SetVelocityInLocalSpace` _projectilemovement _returnvalue_2)
      (set `ProjectileMovementComponent.bRotationFollowsVelocity` true _projectilemovement)
      (set `self.BonusArrow2` null))))

(fn `GrabPressed*`
  (params (WhichHand :type "/Game/Blueprints/Enums/LeftRight Enum" :default "NewEnumerator0") (HandBP :type "/Game/Blueprints/Character/Hands/BP_LeftHand Object Reference"))
  (returns (GrabTransform :type "Transform Structure") (ItemPickedUp :type Boolean) (SecondaryGrab :type Boolean) (LocalGrabLocation :type "Vector Structure"))
  (if (`self.Held?`)
    ;[1 1 1] Grab String
    (set `self.StringHandBP` HandBP)
    (set `self.StringPullHand` WhichHand)
    (set `self.PullingString?` true)
    (set `self.PickUp?` false)
    (set `self.InitialStringGrabOffset` (- (`SceneComponent.K2_GetComponentLocation` (`self.StringSphere`)) (`SceneComponent.K2_GetComponentLocation` (`/Game/Blueprints/Character/Hands/BP_LeftHand.Scene` (`self.StringHandBP`)))))
    (`SceneComponent.SetVisibility` (`self.StringRelease`) false false)
    ;[1 1 1] Put Arrow in Hand
    (`|SpawnActorFromClass` null (`KismetMathLibrary.Conv_VectorToTransform` (0.0 0.0 0.0)) "AlwaysSpawn" "OverrideRootScale")
    (set `self.CurrentArrow` null)
    (`self.SpawnBonusArrows`)
    (else
      ;[1 1 1] Simple Grab
      (set `self.HoldingHand` WhichHand)
      (set `self.Held?` true)
      (set `self.PullingString?` false)
      (set `self.PickUp?` true)))
  (return (`SceneComponent.K2_GetComponentToWorld` (`self.Box`)) (`self.PickUp?`) (`self.PullingString?`) (`KismetMathLibrary.InverseTransformLocation` (`self.GetTransform`) (`SceneComponent.K2_GetComponentLocation` (`self.LSideNook`)))))

(fn `GrabReleased*`
  (params (WhichHand :type "/Game/Blueprints/Enums/LeftRight Enum" :default "NewEnumerator0"))
  (returns (`DropOnRelase?` :type Boolean))
  (bind _projectilemovement (`self.ProjectileMovement`))
  (bind _returnvalue (* (`KismetMathLibrary.FClamp` (`self.Length`) 0.0 35.0) 2.0))
  (if (`|EnumEquality` WhichHand (`self.HoldingHand`))
    ;[1 1 1] Drop Weapon
    (set `self.Held?` false)
    (set `self.PullingString?` false)
    (set `self.Dropped?` true)
    (return (`self.Dropped?`))
    (else
      ;[1 1 1] Fire
      (`|ExecutionSequence`
        (:`then_0`
          (if (`self.PullingString?`)
            (set `self.PullingString?` false)
            (`ActorComponent.SetActive` _projectilemovement true false)
            (`ProjectileMovementComponent.SetVelocityInLocalSpace` _projectilemovement (`KismetMathLibrary.MakeVector` (* (* _returnvalue _returnvalue) 1.0)))
            (set `ProjectileMovementComponent.bRotationFollowsVelocity` true _projectilemovement)
            (`PrimitiveComponent.SetMaterial` (`self.StringRelease`) 0 null)
            (set `self.CurrentArrow` null)
            (`self.FireBonusArrows`)
            (`PlayerController.ClientPlayForceFeedback` (`GameplayStatics.GetPlayerController` 0) "/Game/Blueprints/ViveForces/Force_Left_FireArrow.Force_Left_FireArrow" false "None")))
        (:`then_1`
          (set `self.Dropped?` false)
          (return (`self.Dropped?`)))))))

(fn `HandBeginOverlap*`
  (params (WhichHand :type "/Game/Blueprints/Enums/LeftRight Enum" :default "NewEnumerator0") (HandBP :type "/Game/Blueprints/Character/Hands/BP_LeftHand Object Reference"))
  (returns (Reply :type Boolean) (SelectionMID :type "MaterialInstanceDynamic Object Reference"))
  (if (`self.Held?`)
    (if (not (`|EnumEquality` WhichHand (`self.HoldingHand`)))
      (set `self.StringOverlapHand` WhichHand)
      (`SceneComponent.SetVisibility` (`self.StringRelease`) true false))
    (else
      (bind _output_get (set `self.OverlappingHand` WhichHand))))
  (return true (select `bool` (`self.Held?`) :`false` (select `/Game/Blueprints/Enums/LeftRight` _output_get :`NewEnumerator0` (`self.LNookMID`) :`NewEnumerator1` (`self.RNookMID`)) :`true` (`self.StringMID`))))

(fn `HandEndOverlap*`
  (params (WhichHand :type "/Game/Blueprints/Enums/LeftRight Enum" :default "NewEnumerator0"))
  (returns (NewParam :type Boolean))
  (return false))

(fn `Haptics/Force Feedback`
  (bind _length (`self.Length`))
  (bind _returnvalue (- _length (`self.PrevLength`)))
  (bind _returnvalue_2 (`KismetMathLibrary.FClamp` (/ (`KismetMathLibrary.Abs` _returnvalue) 5.0)))
  (`PlayerController.SetHapticsByValue` (`GameplayStatics.GetPlayerController` 0) (`KismetMathLibrary.FClamp` (+ (/ _length 50.0) (/ _returnvalue 50.0))) _returnvalue_2 (select `/Game/Blueprints/Enums/LeftRight` (`self.StringPullHand`) :`NewEnumerator0` "Left" :`NewEnumerator1` "Right" :!type "EControllerHand Enum"))
  (if (> (`self.TimeAccum`) 0.1)
    (`PlayerController.ClientPlayForceFeedback` (`GameplayStatics.GetPlayerController` 0) (`KismetArrayLibrary.Array_Get` (`self.ForceFeedbacks`) (`KismetMathLibrary.FFloor` (* _returnvalue_2 10.0))) false "None")
    (set `self.TimeAccum` (+ (`self.TimeAccum`) -0.1))
    (else
      (set `self.TimeAccum` (+ (`self.TimeAccum`) (`GameplayStatics.GetWorldDeltaSeconds`)))))
  (set `self.PrevLength` (`self.Length`))
  (return))

(fn `SpawnBonusArrows`
  (if (`self.BonusTripleShot`)
    (`|SpawnActorFromClass` "Bow_C" (`KismetMathLibrary.MakeTransform` (0.0 0.0 0.0)) "AlwaysSpawn" "OverrideRootScale")
    (set `self.BonusArrow1` null)
    (`|SpawnActorFromClass` "Bow_C" (`KismetMathLibrary.MakeTransform` (0.0 0.0 0.0)) "AlwaysSpawn" "OverrideRootScale")
    (set `self.BonusArrow2` null)
    (set `self.BonusTripleShot` false)))

(fn `TriggerPressed*`
  (params (WhichHand :type "/Game/Blueprints/Enums/LeftRight Enum" :default "NewEnumerator0") (HandBP :type "/Game/Blueprints/Character/Hands/BP_LeftHand Object Reference"))
  (returns (GrabTransform :type "Transform Structure") (ItemPickedUp :type Boolean) (SecondaryGrab :type Boolean) (LocalGrabLoction :type "Vector Structure"))
  (return (struct) false false (0.0 0.0 0.0)))

(fn `TriggerReleased*`
  (params (WhichHand :type "/Game/Blueprints/Enums/LeftRight Enum" :default "NewEnumerator0"))
  (returns (`DropOnRelease?` :type Boolean))
  (return false))

(fn `UpdateBonusArrows`
  (bind _returnvalue (+ (`SceneComponent.K2_GetComponentLocation` (`/Game/Blueprints/Character/Hands/BP_LeftHand.Scene` (`self.StringHandBP`))) (`self.InitialStringGrabOffset`)))
  (bind _returnvalue_2 (+ (`SceneComponent.K2_GetComponentLocation` (`/Game/Blueprints/Character/Hands/BP_LeftHand.Scene` (`self.StringHandBP`))) (`self.InitialStringGrabOffset`)))
  (`/Engine/EditorBlueprintResources/StandardMacros.IsValid` null
    (:`Is Valid`
      ;[1 1 1] Position Bonus Arrow 1
      (`self.K2_SetActorTransform` (`KismetMathLibrary.MakeTransform` (+ _returnvalue_2 (- (`self.K2_GetActorLocation`) (`SceneComponent.K2_GetComponentLocation` (`self.Base`)))) (`KismetMathLibrary.MakeRotFromX` (- (+ (`KismetMathLibrary.TransformDirection` (`self.GetTransform`) (+ (0.0 0.0 5.0) (0.0 0.0 0.0))) (`SceneComponent.K2_GetComponentLocation` (select `/Game/Blueprints/Enums/LeftRight` (`self.HoldingHand`) :`NewEnumerator0` (`self.LSideNook`) :`NewEnumerator1` (`self.RSideNook`)))) _returnvalue_2))))
      (`/Engine/EditorBlueprintResources/StandardMacros.IsValid` null
        (:`Is Valid`
          ;[1 1 1] Position Bonus Arrow 2
          (`self.K2_SetActorTransform` (`KismetMathLibrary.MakeTransform` (+ _returnvalue (- (`self.K2_GetActorLocation`) (`SceneComponent.K2_GetComponentLocation` (`self.Base`)))) (`KismetMathLibrary.MakeRotFromX` (- (+ (`KismetMathLibrary.TransformDirection` (`self.GetTransform`) (+ (0.0 0.0 -5.0) (0.0 0.0 0.0))) (`SceneComponent.K2_GetComponentLocation` (select `/Game/Blueprints/Enums/LeftRight` (`self.HoldingHand`) :`NewEnumerator0` (`self.LSideNook`) :`NewEnumerator1` (`self.RSideNook`)))) _returnvalue)))))))))

(fn `UserConstructionScript`
  (bind _returnvalue (`PrimitiveComponent.CreateDynamicMaterialInstance` (`self.StringMesh`) 0 "/Game/Materials/String.String"))
  (set `self.StringMID` _returnvalue)
  (bind _returnvalue_2 (`PrimitiveComponent.CreateDynamicMaterialInstance` (`self.LSideNook`) 0 null))
  (set `self.LNookMID` _returnvalue_2)
  (bind _returnvalue_3 (`PrimitiveComponent.CreateDynamicMaterialInstance` (`self.RSideNook`) 0 null))
  (set `self.RNookMID` _returnvalue_3))