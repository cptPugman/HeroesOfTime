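; Manager Actor that registers zombies and finds the living one nearest to a given location.
; PushZombie fills parallel zombie and alive-flag arrays and increments a count.
; GetNearest scans them by distance from a supplied starting candidate, setting Valid only when the first entry is alive.
; PopZombie removes the zombie entry but only resets its flag, so array indices shift apart and the count never drops.
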(fn `getNearest`
  (params (location :type "Vector Structure") (firstNearest :type "/Game/X-Bot/Punchman Object Reference"))
  (returns (nearestZombie :type "/Game/X-Bot/Punchman Object Reference") (`valid?` :type Boolean))
  (set `self.nearest` firstNearest)
  (for (_array_element _array_index) (`self.ArrayZombies`)
    (if (== _array_index 0)
      (if (!= (`KismetArrayLibrary.Array_Get` (`self.arrayDeadOrAlive`)) 0)
        (set `self.valid?` true)
        (bind _output_get (set `self.nearest` _array_element)))
      (elif (!= (`KismetArrayLibrary.Array_Get` (`self.arrayDeadOrAlive`) _array_index) 0)
        (if (< (`KismetMathLibrary.VSize` (- location (`self.K2_GetActorLocation` _array_element))) (`KismetMathLibrary.VSize` (- location (`self.K2_GetActorLocation` _output_get))))
          (set `self.nearest` _array_element)))))
  (return (`self.nearest`) (`self.valid?`)))

(fn `popZombie`
  (params (id :type Integer))
  (`KismetArrayLibrary.Array_Remove` (`self.ArrayZombies`) id)
  (`KismetArrayLibrary.Array_Set` (`self.arrayDeadOrAlive`) id 0 true))

(fn `pushZombie`
  (params (NewParam :type "/Game/X-Bot/Punchman Object Reference"))
  (returns (id :type Integer))
  (`KismetArrayLibrary.Array_Add` (`self.ArrayZombies`) NewParam)
  (`KismetArrayLibrary.Array_Add` (`self.arrayDeadOrAlive`) 1)
  (bind _output_get (set `self.nZombies` (+ (`self.nZombies`) 1)))
  (return _output_get))

(fn `UserConstructionScript`)