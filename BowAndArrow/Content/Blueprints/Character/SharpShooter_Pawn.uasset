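; SharpShooter_Pawn is a player pawn with VR hands, keyboard movement, arrow shooting and health.
; Child-actor hand Blueprints are cross-linked at BeginPlay, and motion-controller triggers drive their Grab and Release.
; WASD flags polled on Tick move and yaw the pawn, while left click spawns an Arrow below its origin at zero rotation.
; QuitarVida subtracts damage from Vida, updates the TextRender display and destroys the pawn below 1.
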(event `self.ReceiveBeginPlay`
  (`HeadMountedDisplayFunctionLibrary.SetTrackingOrigin` "Floor")
  (`self.RegisterHandBPs`))

(event `Key|MotionController_Left_Trigger`
  (params (Key :type "Key Structure" :default "AnyKey"))
  (bind _lefthandbp (`self.LeftHandBP`))
  (:`Pressed`
    (`/Game/Blueprints/Character/Hands/BP_LeftHand.Grab` _lefthandbp))
  (:`Released`
    (`/Game/Blueprints/Character/Hands/BP_LeftHand.Release` _lefthandbp)))

(event `Key|MotionController_Right_Trigger`
  (params (Key :type "Key Structure" :default "AnyKey"))
  (bind _righthandbp (`self.RightHandBP`))
  (:`Pressed`
    (`/Game/Blueprints/Character/Hands/BP_LeftHand.Grab` _righthandbp))
  (:`Released`
    (`/Game/Blueprints/Character/Hands/BP_LeftHand.Release` _righthandbp)))

(event `Key|S`
  (params (Key :type "Key Structure" :default "AnyKey"))
  (:`Pressed`
    (set `self.sPressed` true))
  (:`Released`
    (set `self.sPressed` false)))

(event `self.ReceiveTick`
  (params (DeltaSeconds :type "Float (single-precision)"))
  (if (`self.wPressedf`)
    (`self.K2_AddActorLocalOffset` self (+ (`self.GetActorForwardVector` self) (`KismetMathLibrary.Conv_RotatorToVector` (`self.rotato`))) false false))
  (if (`self.aPressed`)
    (`self.K2_AddActorLocalRotation` self (struct :`Yaw` -0.5) false false)
    (set `self.rotato` (struct :`Yaw` -0.5)))
  (if (`self.dPressed`)
    (`self.K2_AddActorLocalRotation` self (struct :`Yaw` 0.5) false false)
    (set `self.rotato` (struct :`Yaw` 0.5)))
  (if (`self.sPressed`)
    (`self.K2_AddActorLocalOffset` self (`KismetMathLibrary.NegateVector` (+ (`self.GetActorForwardVector` self) (`KismetMathLibrary.Conv_RotatorToVector` (`self.rotato`)))) false false)))

(event `Key|W`
  (params (Key :type "Key Structure" :default "AnyKey"))
  (:`Pressed`
    (set `self.wPressedf` true))
  (:`Released`
    (set `self.wPressedf` false)))

(event `Key|A`
  (params (Key :type "Key Structure" :default "AnyKey"))
  (:`Pressed`
    (set `self.aPressed` true))
  (:`Released`
    (set `self.aPressed` false)))

(event `Key|D`
  (params (Key :type "Key Structure" :default "AnyKey"))
  (:`Pressed`
    (set `self.dPressed` true))
  (:`Released`
    (set `self.dPressed` false)))

(event `Key|LeftMouseButton`
  (params (Key :type "Key Structure" :default "AnyKey"))
  (:`Pressed`
    (`|SpawnActorFromClass` "/Game/Blueprints/Character/arrow.arrow_C" (`KismetMathLibrary.MakeTransform` (- (`self.K2_GetActorLocation` self) (0.0 0.0 20.0)) (struct) (1.0 1.0 1.0)) "Undefined" "OverrideRootScale")))

(fn `Quitar vida`
  (params (Damage :type Integer))
  (bind _vida (`self.Vida`))
  (bind _output_get (set `self.Vida` (- _vida Damage)))
  (`TextRenderComponent.K2_SetText` (`self.TextRender`) (`KismetTextLibrary.Conv_IntToText` _output_get))
  (if (< _vida 1)
    (`self.K2_DestroyActor`)))

(fn `RegisterHandBPs`
  (bind _lefthandbp (`self.LeftHandBP`))
  (bind _asbp_left_hand (cast `/Game/Blueprints/Character/Hands/BP_LeftHand` (`ChildActorComponent.ChildActor` (`self.LHandChildActor`))))
  (set `self.LeftHandBP` _asbp_left_hand)
  (bind _asbp_right_hand (cast `/Game/Blueprints/Character/Hands/BP_RightHand` (`ChildActorComponent.ChildActor` (`self.RHandChildActor`))))
  (bind _output_get (set `self.RightHandBP` _asbp_right_hand))
  (set `/Game/Blueprints/Character/Hands/BP_LeftHand.OtherHandBlueprint` _output_get _lefthandbp)
  (set `/Game/Blueprints/Character/Hands/BP_LeftHand.OtherHandBlueprint` _lefthandbp (`self.RightHandBP`)))

(fn `UserConstructionScript`
  (`TextRenderComponent.K2_SetText` (`self.TextRender`) (`KismetTextLibrary.Conv_IntToText` (`self.Vida`))))