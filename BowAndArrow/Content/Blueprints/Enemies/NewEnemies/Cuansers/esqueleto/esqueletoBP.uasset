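; Skeleton enemy character whose fist colliders, attached to hand sockets, hit "torreta"-tagged meshes, swapping their material and draining Vida on the Muerte actor.
; With Figherino set, its fists destroy other skeletons.
; Looping timers poll Foc and Fum overlaps to set Burn and Dizzy, which Tick turns into visible particles and quartered walk speed.
; Detection scans GetAllActorsOfClass results, and a startup timer initializes turret materials.
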(event `self.ReceiveBeginPlay`
  (`KismetSystemLibrary.K2_SetTimer` null "cambiarColorTorreta" 0.1)
  (`KismetSystemLibrary.K2_SetTimer` null "burning" 0.1 true)
  (`KismetSystemLibrary.K2_SetTimer` null "humo" 0.1 true))

(event `self.ReceiveTick`
  (params (DeltaSeconds :type "Float (single-precision)"))
  (bind _charactermovement (`self.CharacterMovement`))
  (bind _returnvalue (`self.K2_GetActorLocation` self))
  (bind _maxwalkspeed (`CharacterMovementComponent.MaxWalkSpeed` _charactermovement))
  (if (`self.atack`)
    (bind _outactors (`GameplayStatics.GetAllActorsOfClass` "/Script/Engine.StaticMeshActor"))
    (for _array_element _outactors
      (if (or (`PrimitiveComponent.IsOverlappingActor` (`self.puño derecho`) _array_element) (`PrimitiveComponent.IsOverlappingActor` (`self.puño izquierdo`) _array_element))
        (if (`self.ActorHasTag` _array_element "torreta")
          (`PrimitiveComponent.SetMaterial` (`StaticMeshActor.StaticMeshComponent` _array_element) 3 "/Game/TopViewLevel/3D/Material__48.Material__48")
          (bind _outactors_2 (`GameplayStatics.GetAllActorsOfClass` "/Game/NivelPruebas/Muerte.Muerte_C"))
          (bind _item (`KismetArrayLibrary.Array_Get` _outactors_2))
          (set `/Game/NivelPruebas/Muerte.vida` (- (`/Game/NivelPruebas/Muerte.vida` _item) 0.1) _item))
        (if (`self.figherino`) :!label _label
          (bind _outactors_3 (`GameplayStatics.GetAllActorsOfClass` "esqueletoBP_C"))
          (for _array_element_2 _outactors_3
            (if (or (`PrimitiveComponent.IsOverlappingActor` (`self.puño derecho`) _array_element_2) (`PrimitiveComponent.IsOverlappingActor` (`self.puño izquierdo`) _array_element_2))
              (if (not (== _array_element_2 self))
                (`self.K2_DestroyActor` _array_element_2)))
            (if (`self.dizzy`) :!label _label_2
              (if (not (`self.modSpeed`))
                (set `CharacterMovementComponent.MaxWalkSpeed` (/ _maxwalkspeed 4.0) _charactermovement)
                (set `self.modSpeed` true))
              (elif (`self.modSpeed`)
                (`/Engine/EditorBlueprintResources/StandardMacros.DoOnce` false
                  (:`Completed`
                    (set `CharacterMovementComponent.MaxWalkSpeed` (* 4 _maxwalkspeed) _charactermovement)))))
            (if (`self.burn`)
              (set `self.counter` (+ (`self.counter`) 0.01))
              (`self.K2_SetActorRotation` self (`KismetMathLibrary.FindLookAtRotation` _returnvalue (+ _returnvalue (* (`self.GetActorForwardVector` self) 1000.0))) false)
              (`SceneComponent.SetVisibility` (`self.ParticleSystem`) true false))
            (if (`self.run`)
              _))
          (else
            (goto _label_2)))))
    (else
      (goto _label))))

(event `self.ReceiveActorEndOverlap`
  (params (OtherActor :type "Actor Object Reference"))
  (bind _outactors (`GameplayStatics.GetAllActorsOfClass` "/Game/Blueprints/fum.fum_C"))
  (for _array_element _outactors
    (if (== OtherActor _array_element)
      (set `self.dizzy` false))))

(fn `burning`
  (bind _outactors (`GameplayStatics.GetAllActorsOfClass` "/Game/Blueprints/foc.foc_C"))
  (for _array_element _outactors
    (if (`PrimitiveComponent.IsOverlappingActor` (`self.Mesh`) _array_element)
      (set `self.burn` true))))

(fn `cambiarColorTorreta`
  (bind _outactors (`GameplayStatics.GetAllActorsOfClass` "/Script/Engine.StaticMeshActor"))
  (for _array_element _outactors
    (if (`self.ActorHasTag` _array_element "torreta")
      (`PrimitiveComponent.SetMaterial` (`StaticMeshActor.StaticMeshComponent` _array_element) 3 "/Game/NivelPruebas/Material__59.Material__59"))))

(fn `humo`
  (bind _outactors (`GameplayStatics.GetAllActorsOfClass` "/Game/Blueprints/fum.fum_C"))
  (for _array_element _outactors
    (if (`PrimitiveComponent.IsOverlappingActor` (`self.Mesh`) _array_element)
      (if (`SceneComponent.IsVisible` (`/Game/Blueprints/fum.ParticleSystem` _array_element))
        (set `self.dizzy` true)
        (else
          (set `self.dizzy` false))))))

(fn `UserConstructionScript`
  (bind _mesh (`self.Mesh`))
  (`SceneComponent.K2_AttachTo` (`self.ParticleSystem`) _mesh "Spine1" "SnapToTarget" true)
  (`SceneComponent.K2_AttachTo` (`self.puño derecho`) _mesh "RightHandIndex1" "SnapToTargetIncludingScale" true)
  (`SceneComponent.K2_AttachTo` (`self.puño izquierdo`) _mesh "LeftHandIndex1" "SnapToTargetIncludingScale" true))